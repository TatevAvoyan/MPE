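; BP_Elevator is an elevator actor that builds and removes a vertical shaft made of BP_Shaft segments.
; SpawnShaft spawns one segment per floor at the elevator's X and Y, stacked at fixed height steps from world zero, and stores each in the Shafts array.
; DestroyShaft destroys the stored segments and clears the array.
; The event graph and construction script are empty, so nothing in this file calls either function.
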(fn `DestroyShaft`
  (for _index (range (`self.ShaftFloorsCount`))
    (`self.K2_DestroyActor` (`|GetArrayItem` (`self.Shafts`) _index)))
  (`KismetArrayLibrary.Array_Clear` (`self.Shafts`)))

(fn `SpawnShaft`
  (bind (_returnvalue_x _returnvalue_y) (`KismetMathLibrary.BreakVector` (`self.K2_GetActorLocation`)))
  (for _index (range (`self.ShaftFloorsCount`))
    (bind _returnvalue (`|SpawnActorFromClass` "/Game/EBlueprints/BP_Shaft.BP_Shaft_C" (`KismetMathLibrary.MakeTransform` (`KismetMathLibrary.MakeVector` _returnvalue_x _returnvalue_y (`KismetMathLibrary.Conv_IntToDouble` (* _index 300)))) "AlwaysSpawn" "OverrideRootScale" null null))
    (bind _asbp_shaft (cast `/Game/EBlueprints/BP_Shaft` _returnvalue)
      (:`then`
        (`KismetArrayLibrary.Array_Set` (`self.Shafts`) _index _asbp_shaft true))
      (:`CastFailed`
        (break)))))

(fn `UserConstructionScript`)